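; Controller Blueprint for a BlowStick device, linking it to the game over UDP through a socket client.
; Alt-key shortcuts discover the device IP by broadcast host name, connect, calibrate magnetometer and zero position, start streaming and open the data receiver.
; Each step swaps the socket's receive delegate to its own handler.
; The data handler parses rotation and blow values, firing rotator-change and throttled blow-action dispatchers for other game code.
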(event Custom|UDP_Data_Event
  (params (message :type String) (byteArray :type Array%20of%20Bytes) (IP :type String) (port :type Integer))
  (bind _returnvalue (Utilities|String|ParseIntoArray message " "))
  ;[1 1 1] Start Listening RPYB UDP Data and Setting Variables.
  (Variables|Default|SetBlowStick_Rotator (Math|Rotator|MakeRotator (Math|Conversions|ToFloat(Integer) (Utilities|Array|Get(acopy) _returnvalue)) (Math|Conversions|ToFloat(Integer) (Utilities|Array|Get(acopy) _returnvalue 1)) (Math|Conversions|ToFloat(Integer) (Utilities|Array|Get(acopy) _returnvalue 2))))
  (Variables|Default|SetBlowStick_Blow_Action (Math|Conversions|ToFloat(Integer) (Utilities|Array|Get(acopy) _returnvalue 3)))
  (Variables|Default|SetBlowStick_Blow_Inertialised (Math|Conversions|ToFloat(Integer) (Utilities|Array|Get(acopy) _returnvalue 4)))
  (Variables|Default|SetBlowStick_Blow_Raw (Math|Conversions|ToFloat(Integer) (Utilities|Array|Get(acopy) _returnvalue 5)))
  (Utilities|FlowControl|Sequence
    (:then_0
      ;[1 1 1] BlowActionEvent. You need to connect event to your part of a program.
      (if (!= 0.0 (Variables|Default|GetBlowStick_Blow_Action))
        (Utilities|FlowControl|DoOnce false :!label _label
          (:Completed
            (Utilities|FlowControl|Sequence
              (:then_0
                (Default|CallBlowActionEventDispatcher (Variables|Default|GetBlowStick_Blow_Action)))
              (:then_1
                (Utilities|FlowControl|Delay 0.25)
                (goto _label Reset)))))))
    (:then_1
      (Default|CallRotatorChangeEventDispatcher (Variables|Default|GetBlowStick_Rotator)))))

(event Custom|OnReceiveBrodcastEvent
  (params (message :type String) (byteArray :type Array%20of%20Bytes) (IP :type String) (port :type Integer))
  ;[1 1 1] Connect to BlowStick
  (if (Utilities|Enum|Equal(Enum) message "connected")
    (bind _output_get (Variables|Default|SetBlowStick_Status "Connected"))
    (Development|PrintString _output_get true true "(R=0.073381,G=1.000000,B=0.012392,A=1.000000)")
    (else
      (bind _output_get_2 (Variables|Default|SetBlowStick_Status "Not Connected"))
      (Utilities|FlowControl|DoOnce false
        (:Completed
          (Development|PrintString _output_get_2 true true "(R=1.000000,G=0.000000,B=0.008680,A=1.000000)"))))))

(event Custom|DataEmitEvent
  (params (message :type String) (byteArray :type Array%20of%20Bytes) (IP :type String) (port :type Integer))
  ;[1 1 1] Starting Data Emit on Server
  (if (Utilities|Enum|Equal(Enum) message "data_started")
    (Development|PrintString "Data Started." true true "(R=0.028858,G=1.000000,B=0.000000,A=1.000000)" 3.0)))

(event Custom|OnReceiveUDP
  (params (message :type String) (byteArray :type Array%20of%20Bytes) (IP :type String) (port :type Integer))
  (bind _returnvalue (Utilities|String|ParseIntoArray message " "))
  (bind _output (Utilities|Array|Get(acopy) _returnvalue 2))
  ;[1 1 1] Get BlowStick IP Address from Brodcast
  (Variables|Default|SetTemp_Server_IP_Address IP)
  (Variables|Default|SetUDP_Server_Host_Name _output)
  (Development|PrintString (Utilities|String|Append "Host Name: " _output))
  (if (Utilities|Enum|Equal(Enum) (Variables|Default|GetUDP_Server_Host_Name) (Variables|Default|GetUDP_Desired_Host_Name))
    (Variables|Default|SetUDP_Server_IP_Address (Variables|Default|GetTemp_Server_IP_Address))
    (Development|PrintString (Utilities|String|Append "DesiredHostFound: " (Variables|Default|GetUDP_Desired_Host_Name)))
    (else
      (Variables|Default|SetUDP_Server_IP_Address "False"))))

(event Custom|CustomEventMCalibrate
  (params (message :type String) (byteArray :type Array%20of%20Bytes) (IP :type String) (port :type Integer))
  ;[1 1 1] Magnetometer Calibration
  (if (Utilities|Enum|Equal(Enum) message "magnetometer_calibration_finished")
    (Development|PrintString "Magnetometer Calibration Finished" true true "(R=0.028858,G=1.000000,B=0.000000,A=1.000000)" 3.0)))

(event Custom|CustomEventZerroCalibration
  (params (message :type String) (byteArray :type Array%20of%20Bytes) (IP :type String) (port :type Integer))
  ;[1 1 1] Zero Position Calibration
  (if (Utilities|Enum|Equal(Enum) message "zero_calibration_finished")
    (Development|PrintString "Zero Calibration Finished" true true "(R=0.028858,G=1.000000,B=0.000000,A=1.000000)" 3.0)))

(event EventBeginPlay)

(event Collision|EventActorBeginOverlap
  (params (OtherActor :type Actor%20Object%20Reference)))

(event Input|KeyboardEvents|AltR
  (params (Key :type Key%20Structure))
  (bind _returnvalue (Class|SocketClientHandler|GetSocketClientTarget))
  (bind _blowstick_udp_broadcast_port (Variables|Default|GetBlowStick_UDP_Broadcast_Port))
  (:Pressed
    ;[1 1 1] Get BlowStick IP Address from Brodcast
    (EventDispatchers|UnbindallEventsfromOnreceiveUDPMessageEventDelegate _returnvalue)
    (Class|SocketClientBPLibrary|CloseSocketClientConnection _returnvalue)
    (bind _returnvalue_2 (Class|SocketClientBPLibrary|GetLocalIP))
    (Development|PrintString _returnvalue_2)
    (Class|SocketClientBPLibrary|SocketClientInitUDPReceiver (Class|SocketClientHandler|GetSocketClientTarget) _returnvalue_2 _blowstick_udp_broadcast_port)
    (Development|PrintString (Utilities|String|Append "UDP Receiver Started on port " (Utilities|String|ToString(Integer) _blowstick_udp_broadcast_port)))
    (Utilities|FlowControl|Delay (Variables|Default|GetWaiting_UDP_Response_Delay))
    (EventDispatchers|BindEventtoOnreceiveUDPMessageEventDelegate (Class|SocketClientHandler|GetSocketClientTarget) (delegate Custom|OnReceiveUDP))))

(event Input|KeyboardEvents|AltC
  (params (Key :type Key%20Structure))
  (:Pressed
    ;[1 1 1] Connect to BlowStick
    (Development|PrintString "Connecting to BlowStick...")
    (EventDispatchers|UnbindallEventsfromOnreceiveUDPMessageEventDelegate (Class|SocketClientHandler|GetSocketClientTarget))
    (EventDispatchers|BindEventtoOnreceiveUDPMessageEventDelegate (Class|SocketClientHandler|GetSocketClientTarget) (delegate Custom|OnReceiveBrodcastEvent))
    (Class|SocketClientBPLibrary|SocketClientSendUDPMessage (Class|SocketClientHandler|GetSocketClientTarget) (Variables|Default|GetUDP_Server_IP_Address) (Variables|Default|GetBlowStick_UDP_Broadcast_Send_Port) "connect" 0 false)))

(event Input|KeyboardEvents|AltM
  (params (Key :type Key%20Structure))
  (:Pressed
    ;[1 1 1] Magnetometer Calibration
    (Development|PrintString "Magnetometer Calibration Started")
    (EventDispatchers|UnbindallEventsfromOnreceiveUDPMessageEventDelegate (Class|SocketClientHandler|GetSocketClientTarget))
    (EventDispatchers|BindEventtoOnreceiveUDPMessageEventDelegate (Class|SocketClientHandler|GetSocketClientTarget) (delegate Custom|CustomEventMCalibrate))
    (Class|SocketClientBPLibrary|SocketClientSendUDPMessage (Class|SocketClientHandler|GetSocketClientTarget) (Variables|Default|GetUDP_Server_IP_Address) (Variables|Default|GetBlowStick_UDP_Broadcast_Send_Port) "calibrate_magnetometer" 0 false)))

(event Input|KeyboardEvents|AltD
  (params (Key :type Key%20Structure))
  (:Pressed
    ;[1 1 1] Starting Data Emit on Server
    (Development|PrintString "Starting RPYB Data on Server...")
    (EventDispatchers|UnbindallEventsfromOnreceiveUDPMessageEventDelegate (Class|SocketClientHandler|GetSocketClientTarget))
    (EventDispatchers|BindEventtoOnreceiveUDPMessageEventDelegate (Class|SocketClientHandler|GetSocketClientTarget) (delegate Custom|DataEmitEvent))
    (Class|SocketClientBPLibrary|SocketClientSendUDPMessage (Class|SocketClientHandler|GetSocketClientTarget) (Variables|Default|GetUDP_Server_IP_Address) (Variables|Default|GetBlowStick_UDP_Broadcast_Send_Port) "start_data" 0 false)))

(event Input|KeyboardEvents|AltZ
  (params (Key :type Key%20Structure))
  (:Pressed
    ;[1 1 1] Zero Position Calibration
    (Development|PrintString "Zerro Calibration Started")
    (EventDispatchers|UnbindallEventsfromOnreceiveUDPMessageEventDelegate (Class|SocketClientHandler|GetSocketClientTarget))
    (EventDispatchers|BindEventtoOnreceiveUDPMessageEventDelegate (Class|SocketClientHandler|GetSocketClientTarget) (delegate Custom|CustomEventZerroCalibration))
    (Class|SocketClientBPLibrary|SocketClientSendUDPMessage (Class|SocketClientHandler|GetSocketClientTarget) (Variables|Default|GetUDP_Server_IP_Address) (Variables|Default|GetBlowStick_UDP_Broadcast_Send_Port) "calibrate_zero" 0 false)))

(event Input|KeyboardEvents|AltP
  (params (Key :type Key%20Structure))
  (bind _returnvalue (Class|SocketClientHandler|GetSocketClientTarget))
  (bind _blowstick_receive_rpyb_port (Variables|Default|GetBlowStick_Receive_RPYB_Port))
  (:Pressed
    ;[1 1 1] Start Listening RPYB UDP Data and Setting Variables.
    (EventDispatchers|UnbindallEventsfromOnreceiveUDPMessageEventDelegate _returnvalue)
    (Class|SocketClientBPLibrary|CloseSocketClientConnection _returnvalue)
    (bind _returnvalue_2 (Class|SocketClientBPLibrary|GetLocalIP))
    (Development|PrintString _returnvalue_2)
    (Class|SocketClientBPLibrary|SocketClientInitUDPReceiver (Class|SocketClientHandler|GetSocketClientTarget) _returnvalue_2 _blowstick_receive_rpyb_port)
    (Development|PrintString (Utilities|String|Append "UDP Receiver Started on port " (Utilities|String|ToString(Integer) _blowstick_receive_rpyb_port)))
    (Utilities|FlowControl|Delay (Variables|Default|GetWaiting_UDP_Response_Delay))
    (EventDispatchers|BindEventtoOnreceiveUDPMessageEventDelegate (Class|SocketClientHandler|GetSocketClientTarget) (delegate Custom|UDP_Data_Event))))

(fn ConstructionScript)