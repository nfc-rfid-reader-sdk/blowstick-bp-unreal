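; Debug test actor that exercises the player-to-blowstick mapping in BP_BlowStick_Controller.
; BeginPlay caches the first controller found in the level.
; Pressing T prints each BlowStickStructure entry's name and player number, queries GetPlayerNumberFromBlowstickIndex, assigns a player via SetPlayerNumberAtBlowstickIndex, then repeats the query.
; On-screen messages report whether each lookup found a player, with the index shown after the assignment.
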(event EventBeginPlay
  (bind _outactors (Actor|GetAllActorsOfClass "/Game/blowstick_system_unreal/blowstick-bp-unreal/BP_BlowStick_Controller.BP_BlowStick_Controller_C"))
  (Variables|Default|SetBlowStickBP (Utilities|Array|Get(acopy) _outactors)))

(event Collision|EventActorBeginOverlap
  (params (OtherActor :type Actor%20Object%20Reference)))

(event EventTick
  (params (DeltaSeconds :type Float%20%28single-precision%29)))

(event Input|KeyboardEvents|T
  (params (Key :type Key%20Structure))
  (:Pressed
    (for _array_element (Variables|/Game/blowstick_system_unreal/blowstick-bp-unreal/BP_BlowStick_Controller.BP_BlowStick_Controller_C|GetBlowStickStructure (Variables|Default|GetBlowStickBP))
      (Development|PrintString (Utilities|String|Append (.name _array_element) "@Player " (Utilities|String|ToString(Integer) (.playernumber _array_element))) true true "(R=0.000000,G=1.000000,B=0.069329,A=1.000000)" 1e+01))
    (bind _founded_ (Default|GetPlayerNumberfromBlowstickIndex (Variables|Default|GetBlowStickBP) 1))
    (if _founded_
      (Development|PrintString "PlayerFounded" true true "(R=0.000000,G=1.000000,B=0.119997,A=1.000000)" 5.0)
      (else
        (Development|PrintString "PlayerNotFounded" true true "(R=0.000000,G=1.000000,B=0.119997,A=1.000000)" 5.0)))
    (Default|SetPlayerNumberatBlowstickIndex (Variables|Default|GetBlowStickBP) 0 1)
    (bind (_founded__2 _blowstickindex) (Default|GetPlayerNumberfromBlowstickIndex (Variables|Default|GetBlowStickBP) 1))
    (if _founded__2
      (Development|PrintString (Utilities|String|Append "PlayerFounded@Index " (Utilities|String|ToString(Integer) _blowstickindex)) true true "(R=0.000000,G=1.000000,B=0.119997,A=1.000000)" 5.0)
      (else
        (Development|PrintString "PlayerNotFounded" true true "(R=1.000000,G=0.000000,B=0.028497,A=1.000000)" 5.0)))))

(fn ConstructionScript)